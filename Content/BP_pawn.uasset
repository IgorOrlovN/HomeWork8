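; BP_pawn is a player pawn that slides sideways along world Y and spawns the ball at play start.
; Two MoveRight axis handlers apply a fixed per-call offset by input sign, without sweep or delta-time scaling.
; SpawnBall, called on BeginPlay, creates BP_Ball at the capsule's location.
; It then sets PlayingBall to None rather than the spawned actor before binding OnDead on it, with no handler logic shown.
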(event EventBeginPlay
  (CallFunction|SpawnBall))

(event Collision|EventActorBeginOverlap
  (params (OtherActor :type Actor%20Object%20Reference)))

(event EventTick
  (params (DeltaSeconds :type Float%20%28single-precision%29)))

(event Input|AxisEvents|InputAxisMoveRight
  (params (AxisValue :type Float%20%28single-precision%29))
  (if (> AxisValue 0.0)
    (Transformation|AddActorWorldOffset "0,10.000000, 0")))

(event Input|AxisEvents|InputAxisMoveRight
  (params (AxisValue :type Float%20%28single-precision%29))
  (if (< AxisValue 0.0)
    (Transformation|AddActorWorldOffset "0,-10.000000, 0")))

(fn ConstructionScript)

(fn SpawnBall
  (Game|SpawnActorfromClass "/Game/BP_Ball.BP_Ball_C" (Math|Transform|MakeTransform (Transformation|GetWorldLocation (Variables|Default|GetCapsule)) "0, 0, 0" "1,1,1") "AlwaysSpawn" 0 0)
  (bind _output_get (Variables|Default|SetPlayingBall 0))
  (EventDispatchers|BindEventtoOnDead _output_get (EventDispatchers|CreateEvent :!event SpawnBall))
  (return))